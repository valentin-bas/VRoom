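; GBScreen_BP is a Game Boy screen Blueprint that relays player input for the eight handheld buttons: D-pad, A, B, Start and Select.
; Each input action sets IsPressed on press or release, then passes it to that button's ChangeState function, which is defined outside these graphs.
; The Blueprint holds no screen rendering logic, and its construction script is empty.
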(event `InputAction|GBUpKey`
  (:`Pressed`
    (set `self.IsPressed` true)
    (`self.UpButtonChangeState` (`self.IsPressed`) :!label _label))
  (:`Released`
    (set `self.IsPressed` false)
    (goto _label)))

(event `InputAction|GBAKey`
  (:`Pressed`
    (set `self.IsPressed` true)
    (`self.AButtonChangeState` (`self.IsPressed`) :!label _label_2))
  (:`Released`
    (set `self.IsPressed` false)
    (goto _label_2)))

(event `InputAction|GBDownKey`
  (:`Pressed`
    (set `self.IsPressed` true)
    (`self.DownButtonChangeState` (`self.IsPressed`) :!label _label_3))
  (:`Released`
    (set `self.IsPressed` false)
    (goto _label_3)))

(event `InputAction|GBBKey`
  (:`Pressed`
    (set `self.IsPressed` true)
    (`self.BButtonChangeState` (`self.IsPressed`) :!label _label_4))
  (:`Released`
    (set `self.IsPressed` false)
    (goto _label_4)))

(event `InputAction|GBLeftKey`
  (:`Pressed`
    (set `self.IsPressed` true)
    (`self.LeftButtonChangeState` (`self.IsPressed`) :!label _label_5))
  (:`Released`
    (set `self.IsPressed` false)
    (goto _label_5)))

(event `InputAction|GBStartKey`
  (:`Pressed`
    (set `self.IsPressed` true)
    (`self.StartButtonChangeState` (`self.IsPressed`) :!label _label_6))
  (:`Released`
    (set `self.IsPressed` false)
    (goto _label_6)))

(event `InputAction|GBSelectKey`
  (:`Pressed`
    (set `self.IsPressed` true)
    (`self.SelectButtonChangeState` (`self.IsPressed`) :!label _label_7))
  (:`Released`
    (set `self.IsPressed` false)
    (goto _label_7)))

(event `InputAction|GBRightKey`
  (:`Pressed`
    (set `self.IsPressed` true)
    (`self.RightButtonChangeState` (`self.IsPressed`) :!label _label_8))
  (:`Released`
    (set `self.IsPressed` false)
    (goto _label_8)))

(fn `UserConstructionScript`)